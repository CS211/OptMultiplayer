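; BP_Matchmaker is a Blueprint that automatically matches the local player into a multiplayer session on BeginPlay.
; It searches for non-LAN sessions and joins the first result.
; If none are found, it creates a two-connection session with LAN enabled, unlike the search, and opens the LevelString level as a listen server.
; Search and creation failures only print a message.
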(event EventBeginPlay
  (bind _results (|FindSessions (Game|GetPlayerController 0) 10 false)
    (:OnSuccess
      (if (== (Utilities|Array|Length _results) 0)
        (|Session (Game|GetPlayerController 0) 2 true
          (:OnSuccess
            (Game|OpenLevel(byName) (Variables|Default|GetLevelString) true "listen"))
          (:OnFailure
            (Development|PrintString "Create Session Fail")))
        (else
          (|JoinSession (Game|GetPlayerController 0) (Utilities|Array|Get(acopy) _results)))))
    (:OnFailure
      (Development|PrintString "SessionFails"))))

(fn ConstructionScript)